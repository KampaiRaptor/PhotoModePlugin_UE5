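; Photo mode pawn that frames shots with a cine camera on a spring arm, takes high-res PNG screenshots and shows them in its widget.
; Enhanced Input drives look, clamped socket-offset panning and cycling through filmback, zoom, focus, aperture, time dilation and filter categories, with gamepad step throttling.
; Exiting, locked briefly after spawn, resets time, blends back to the player pawn and destroys this one.
; A HighResShot console path for final builds is left unwired.
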(event `self.ReceiveBeginPlay`
  (bind _returnvalue (pcsubsystem `EnhancedInputLocalPlayerSubsystem` (`GameplayStatics.GetPlayerController` 0)))
  (set `SpringArmComponent.TargetArmLength` (`self.DistanceFromTarget`) (`self.SpringArm`))
  ;[0.01042 0.01042 0.01042 1 32] Setup Movement Input
  (`/Engine/EditorBlueprintResources/StandardMacros.IsValid` _returnvalue
    (:`Is Valid`
      (`EnhancedInputSubsystemInterface.AddMappingContext` _returnvalue "/Game/PhotoMode/Input/PM_CameraMappingContext.PM_CameraMappingContext" 0 (struct))
      ;[0.01042 0.01042 0.01042 1 32] Setup Widget
      (bind _returnvalue_2 (`|CreateWidget` "/Game/PhotoMode/Widgets/WBT_PhotoModeWidget.WBT_PhotoModeWidget_C"))
      (bind _output_get (set `self.PM_Widget` _returnvalue_2))
      (`UserWidget.AddToViewport` _output_get 0)
      (`self.ChangeCameraValues` 0.0) ; Setup text for first camera category
      ;[0.01042 0.01042 0.01042] Prevent spamming transition between pawns
      (`KismetSystemLibrary.Delay` 1.0)
      (`self.UnlockReturn`))))

(event `EnhancedInput|/Game/PhotoMode/Input/IA_PM_Look`
  (params (ActionValue :type "Vector2D Structure") (ElapsedSeconds :type "Float (double-precision)") (TriggeredSeconds :type "Float (double-precision)") (InputAction :type "InputAction Object Reference" :default "/Game/PhotoMode/Input/IA_PM_Look.IA_PM_Look"))
  (bind (_x _y) (`KismetMathLibrary.BreakVector2D` ActionValue))
  ;[0.01042 0.01042 0.01042 1 32] Look
  (:`Triggered`
    (`self.AddControllerYawInput` _x)
    (`self.AddControllerPitchInput` (`KismetMathLibrary.SelectFloat` (* _y -1.0) _y (`self.bIsVerticalReversed`)))))

(event `EnhancedInput|/Game/PhotoMode/Input/IA_PM_Movement`
  (params (ActionValue :type "Vector2D Structure") (ElapsedSeconds :type "Float (double-precision)") (TriggeredSeconds :type "Float (double-precision)") (InputAction :type "InputAction Object Reference" :default "/Game/PhotoMode/Input/IA_PM_Movement.IA_PM_Movement"))
  ;[0.01042 0.01042 0.01042 1 32] Movement
  (:`Triggered`
    (`self.AdjustLocation` ActionValue -60.0 60.0)))

(event `EnhancedInput|/Game/PhotoMode/Input/IA_PM_TakeShot`
  (params (ActionValue :type Boolean) (ElapsedSeconds :type "Float (double-precision)") (TriggeredSeconds :type "Float (double-precision)") (InputAction :type "InputAction Object Reference" :default "/Game/PhotoMode/Input/IA_PM_TakeShot.IA_PM_TakeShot"))
  (bind (_resolution _int_resolution) (`self.GetNewPhotoResolution` 1.0))
  ;[0.01042 0.01042 0.01042 1 32] Take Photo
  (:`Started`
    (`/Game/PhotoMode/Widgets/WBT_PhotoModeWidget.TakeShotAnimation` (`self.PM_Widget`))
    (`GameplayStatics.PlaySound2D` "/Game/PhotoMode/Assets/Sounds/CUE_CameraClick.CUE_CameraClick" 1.0 1.0 0.0 null null)
    (set `self.CurrentPhoto` (`KismetStringLibrary.Concat_StrStr` (`KismetSystemLibrary.GetProjectSavedDirectory`) (`self.GetNewPhotoName`) ".png"))
    ;;[0 0.02083 0.01472] In-Editor testing
    (`AutomationBlueprintFunctionLibrary.TakeHighResScreenshot` _int_resolution _int_resolution (`self.CurrentPhoto`) null)
    (`KismetSystemLibrary.Delay` 2.0)
    (bind _returnvalue (`KismetRenderingLibrary.ImportFileAsTexture2D` (`self.CurrentPhoto`)))
    (`/Game/PhotoMode/Widgets/WBT_PhotoModeWidget.LoadPhotoAnimation` (`self.PM_Widget`) _returnvalue)))

(event `EnhancedInput|/Game/PhotoMode/Input/IA_PM_ChangeCameraValue`
  (params (ActionValue :type "Float (double-precision)") (ElapsedSeconds :type "Float (double-precision)") (TriggeredSeconds :type "Float (double-precision)") (InputAction :type "InputAction Object Reference" :default "/Game/PhotoMode/Input/IA_PM_ChangeCameraValue.IA_PM_ChangeCameraValue"))
  ;[0.01042 0.01042 0.01042 1 32] Camera Settings
  (:`Triggered`
    (`self.ChangeCameraValues` ActionValue)))

(event `EnhancedInput|/Game/PhotoMode/Input/IA_PM_ChangeCameraValueGamepad`
  (params (ActionValue :type "Float (double-precision)") (ElapsedSeconds :type "Float (double-precision)") (TriggeredSeconds :type "Float (double-precision)") (InputAction :type "InputAction Object Reference" :default "/Game/PhotoMode/Input/IA_PM_ChangeCameraValueGamepad.IA_PM_ChangeCameraValueGamepad"))
  ;[0.01042 0.01042 0.01042 1 32] Camera Settings
  (:`Triggered`
    ;;[0.01042 0.01042 0.01042] This prevents Gamepad for scrolling through categories too quickly
    (if (`self.GetSingleStepCategories`)
      (`/Engine/EditorBlueprintResources/StandardMacros.DoOnce` false :!label _label
        (:`Completed`
          (`|ExecutionSequence`
            (:`then_0`
              (`KismetSystemLibrary.Delay` 0.2)
              (goto _label :!via `Reset`))
            (:`then_1`
              _)))))
    (`self.ChangeCameraValues` ActionValue true)))

(event `EnhancedInput|/Game/PhotoMode/Input/IA_PM_ChangeCameraCategory`
  (params (ActionValue :type "Float (double-precision)") (ElapsedSeconds :type "Float (double-precision)") (TriggeredSeconds :type "Float (double-precision)") (InputAction :type "InputAction Object Reference" :default "/Game/PhotoMode/Input/IA_PM_ChangeCameraCategory.IA_PM_ChangeCameraCategory"))
  ;[0.01042 0.01042 0.01042 1 32] Camera Settings
  (:`Started`
    (`self.Change Camera Category` ActionValue)))

(event `EnhancedInput|/Game/PhotoMode/Input/IA_PM_SwitchCameraBack`
  (params (ActionValue :type Boolean) (ElapsedSeconds :type "Float (double-precision)") (TriggeredSeconds :type "Float (double-precision)") (InputAction :type "InputAction Object Reference" :default "/Game/PhotoMode/Input/IA_PM_SwitchCameraBack.IA_PM_SwitchCameraBack"))
  ;[0.01042 0.01042 0.01042 1 32] Return to original pawn
  (:`Started`
    (`/Engine/EditorBlueprintResources/StandardMacros.DoOnce` true :!label _label_2
      (:`Completed`
        ;;[0.01042 0.01042 0.01042] Reset time and remove mapping context
        (`GameplayStatics.SetGlobalTimeDilation` 1.0)
        (`EnhancedInputSubsystemInterface.RemoveMappingContext` (pcsubsystem `EnhancedInputLocalPlayerSubsystem` (`GameplayStatics.GetPlayerController` 0)) "/Game/PhotoMode/Input/PM_CameraMappingContext.PM_CameraMappingContext" (struct))
        (`PlayerController.SetViewTargetWithBlend` (`GameplayStatics.GetPlayerController` 0) (`self.PlayerPawn`) 0.5 "VTBlend_Linear" 0.0 false)
        (`/Game/PhotoMode/Widgets/WBT_PhotoModeWidget.DestroyWidget` (`self.PM_Widget`))
        (`KismetSystemLibrary.Delay` 0.5)
        ;;[0.01042 0.01042 0.01042] Return back to original pawn
        (`Controller.Possess` (`GameplayStatics.GetPlayerController` 0) (`self.PlayerPawn`))
        (`self.K2_DestroyActor`)))))

(event `UnlockReturn`
  ;[0.01042 0.01042 0.01042 1 32] Return to original pawn
  (goto _label_2 :!via `Reset`))

(fn `AdjustLocation`
  (params (Input :type "Vector2D Structure") (Min :type "Float (double-precision)" :default -30.0) (Max :type "Float (double-precision)" :default 30.0))
  (locals (SpeedMultiplayer :type "Float (double-precision)" :default 0.2))
  (bind (_x _y) (`KismetMathLibrary.BreakVector2D` Input))
  (bind _speedmultiplayer (`local.SpeedMultiplayer`))
  (bind _springarm (`self.SpringArm`))
  (bind (_socketoffset_x _socketoffset_y _socketoffset_z) (`KismetMathLibrary.BreakVector` (`SpringArmComponent.SocketOffset` _springarm)))
  (bind (_x_2 _y_2) (`KismetMathLibrary.BreakVector2D` (`KismetMathLibrary.MakeVector2D` (* _x _speedmultiplayer) (* _y _speedmultiplayer))))
  (set `SpringArmComponent.SocketOffset` (`KismetMathLibrary.MakeVector` 0.0 (`KismetMathLibrary.FClamp` (+ _socketoffset_y (* _x_2 -1.0)) (`local.Min`) (`local.Max`)) (`KismetMathLibrary.FClamp` (+ _socketoffset_z _y_2) (`local.Min`) (`local.Max`))) _springarm) ; Add offset to Spring arm
)

(fn `Change Camera Category`
  (params (Input :type "Float (double-precision)"))
  (bind _returnvalue (+ (`self.CurrentCameraMode`) 1))
  (bind _returnvalue_2 (- (`self.CurrentCameraMode`) 1))
  (if (> Input 0.0)
    ;[0.01703 0.0625 0.04042] Move one category up, clamp back to start if you go over all categories
    (if (< _returnvalue 6)
      (set `self.CurrentCameraMode` (cast `/Game/PhotoMode/Assets/E_PhotoMode` _returnvalue))
      (else
        (set `self.CurrentCameraMode` "NewEnumerator4")))
    (else
      ;[0.01481 0.01654 0.0625] Move one category down, clamp to last if you go over all categories
      (if (== _returnvalue_2 255)
        (set `self.CurrentCameraMode` "NewEnumerator5")
        (else
          (set `self.CurrentCameraMode` (cast `/Game/PhotoMode/Assets/E_PhotoMode` _returnvalue_2))))))
  (`self.ChangeCameraValues` 0.0) ; Just to update widget text
)

(fn `ChangeCameraValues`
  (params (AddedValue :type "Float (double-precision)") (bIsGamepad :type Boolean))
  (bind _cinecamera (`self.CineCamera`))
  (bind _cinecamera_2 (`self.CineCamera`))
  (bind _cinecamera_3 (`self.CineCamera`))
  (bind _output (`|GetArrayItem` (`self.CameraPresetList`) (`self.CurrentCameraPreset`)))
  (bind (_focussettings_focusmethod _focussettings_manualfocusdistance _focussettings_trackingfocussettings _focussettings_bsmoothfocuschanges _focussettings_focussmoothinginterpspeed _focussettings_focusoffset) (break `CameraFocusSettings` (`CineCameraComponent.FocusSettings` _cinecamera_2)))
  (bind _returnvalue (`KismetMathLibrary.FClamp` (+ (`GameplayStatics.GetGlobalTimeDilation`) (* (`local.AddedValue`) (`KismetMathLibrary.SelectFloat` 0.005 0.01 (`local.bIsGamepad`)))) 0.0 2.0))
  (bind _returnvalue_2 (+ _focussettings_manualfocusdistance (* (`local.AddedValue`) (* _focussettings_manualfocusdistance (`KismetMathLibrary.SelectFloat` 0.005 0.01 (`local.bIsGamepad`))))))
  (switch `/Game/PhotoMode/Assets/E_PhotoMode` (`self.CurrentCameraMode`)
    (:`NewEnumerator4`
      ;[0.01042 0.01042 0.01042 1 32] Change camera type
      (if (== (`local.AddedValue`) 0.0)
        _
        (elif (> (`local.AddedValue`) 0.0)
          (set `self.CurrentCameraPreset` (`KismetMathLibrary.Clamp` (+ (`self.CurrentCameraPreset`) 1) 0 (`KismetArrayLibrary.Array_LastIndex` (`self.CameraPresetList`))))
          (else
            (set `self.CurrentCameraPreset` (`KismetMathLibrary.Clamp` (- (`self.CurrentCameraPreset`) 1) 0 (`KismetArrayLibrary.Array_LastIndex` (`self.CameraPresetList`)))))))
      (`CineCameraComponent.SetFilmbackPresetByName` (`self.CineCamera`) _output)
      (`self.UpdateWidgetText` "NewEnumerator4" 0.0 _output))
    (:`NewEnumerator0`
      ;[0.01042 0.01042 0.01042 1 32] Zoom
      (bind _output_get (set `CineCameraComponent.CurrentFocalLength` (+ (`CineCameraComponent.CurrentFocalLength` _cinecamera_3) (* (`local.AddedValue`) (`KismetMathLibrary.SelectFloat` 0.3 2.0 (`local.bIsGamepad`)))) _cinecamera_3))
      (`self.UpdateWidgetText` "NewEnumerator0" _output_get))
    (:`NewEnumerator1`
      ;[0.01042 0.01042 0.01042 1 32] Focus Distance
      (set `CineCameraComponent.FocusSettings` (make `CameraFocusSettings` _focussettings_focusmethod _returnvalue_2 _focussettings_trackingfocussettings _focussettings_bsmoothfocuschanges _focussettings_focussmoothinginterpspeed _focussettings_focusoffset) _cinecamera_2)
      (`self.UpdateWidgetText` "NewEnumerator1" _returnvalue_2))
    (:`NewEnumerator2`
      ;[0.01042 0.01042 0.01042 1 32] Blur
      (bind _output_get_2 (set `CineCameraComponent.CurrentAperture` (+ (`CineCameraComponent.CurrentAperture` _cinecamera) (* (`local.AddedValue`) (`KismetMathLibrary.SelectFloat` 0.01 1.0 (`local.bIsGamepad`)))) _cinecamera))
      (`self.UpdateWidgetText` "NewEnumerator2" _output_get_2))
    (:`NewEnumerator3`
      ;[0.01042 0.01042 0.01042 1 32] Time dilatation
      (`GameplayStatics.SetGlobalTimeDilation` _returnvalue)
      (`self.UpdateWidgetText` "NewEnumerator3" _returnvalue))
    (:`NewEnumerator5`
      ;[0.01042 0.01042 0.01042 1 32] Scroll through filters
      (if (== (`local.AddedValue`) 0.0)
        _
        (elif (> (`local.AddedValue`) 0.0)
          (set `self.CurrentFilter` (`KismetMathLibrary.Clamp` (+ (`self.CurrentFilter`) 1) 0 (`KismetArrayLibrary.Array_LastIndex` (`self.FiltersList`))))
          (else
            (set `self.CurrentFilter` (`KismetMathLibrary.Clamp` (- (`self.CurrentFilter`) 1) 0 (`KismetArrayLibrary.Array_LastIndex` (`self.FiltersList`)))))))
      (set `CameraComponent.PostProcessSettings` (make `PostProcessSettings` :`ColorGradingLUT` (`|GetArrayItem` (`self.FiltersList`) (`self.CurrentFilter`))) (`self.CineCamera`))
      (`self.UpdateWidgetText` "NewEnumerator5" (`KismetMathLibrary.Conv_IntToDouble` (`self.CurrentFilter`))))))

(fn `GetNewPhotoName`
  (returns (ReturnValue :type String))
  (bind (_returnvalue_year _returnvalue_month _returnvalue_day _returnvalue_hour _returnvalue_minute _returnvalue_second) (`KismetMathLibrary.BreakDateTime` (`KismetMathLibrary.Now`)))
  (return (`KismetStringLibrary.Concat_StrStr` (`self.AlbumName`) "_" (`KismetStringLibrary.Concat_StrStr` (`KismetStringLibrary.Conv_IntToString` _returnvalue_hour) "_" (`KismetStringLibrary.Conv_IntToString` _returnvalue_minute) "_" (`KismetStringLibrary.Conv_IntToString` _returnvalue_second)))))

(fn `GetNewPhotoResolution`
  (params (`Scale Multiplayer` :type "Float (double-precision)" :default 1.0))
  (returns (Resolution :type String) (Int_Resolution :type Integer))
  (bind _returnvalue (* `Scale Multiplayer` 1024.0))
  (bind _returnvalue_2 (`KismetStringLibrary.Conv_DoubleToString` _returnvalue))
  (return (`KismetStringLibrary.Concat_StrStr` _returnvalue_2 "x" _returnvalue_2) (`KismetMathLibrary.FTrunc` _returnvalue)))

(fn `GetSingleStepCategories`
  (returns (ReturnValue :type Boolean))
  (return (or (`|EnumEquality` (`self.CurrentCameraMode`) "NewEnumerator4") (`|EnumEquality` (`self.CurrentCameraMode`) "NewEnumerator5"))))

(fn `UserConstructionScript`)